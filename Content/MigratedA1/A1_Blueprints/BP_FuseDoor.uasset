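; BP_FuseDoor is a door actor that opens once through its OpenDoor function, with no closing logic.
; A boolean guard lets the first call snap the door open with an instant local rotation and trigger a 2D sound.
; It then casts the player's pawn to A2Character and, on success, sets the first material slot on StaticMesh.
; The event graph has no active logic, so opening relies on an external call.
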(event `self.ReceiveTick`
  (params (DeltaSeconds :type "Float (single-precision)")))

(fn `Open Door`
  (if (== (`self.doorIsOpen`) false)
    (`self.K2_AddActorLocalRotation` (struct :`Yaw` -90.0))
    (set `self.doorIsOpen` true)
    (`GameplayStatics.PlaySound2D` null)
    (cast `A2Character` (`Controller.K2_GetPawn` (`GameplayStatics.GetPlayerController` 0)))
    (`PrimitiveComponent.SetMaterial` (`self.StaticMesh`) 0 null)))

(fn `UserConstructionScript`)