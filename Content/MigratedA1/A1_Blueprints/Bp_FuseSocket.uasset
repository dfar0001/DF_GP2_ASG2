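; Fuse socket puzzle actor where the player places a fuse and rotates it to open doors.
; Box overlap toggles input: E shows the fuse mesh if the pawn holds exactly one fuse, and F turns a placed fuse by 90 degrees.
; Tick polls the rotation count and, at two, calls OpenDoor on all actors of a class and changes a mesh material.
; Leaving the box hides the fuse and resets the count, but not the placed flag.
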(event `self.Box.OnComponentBeginOverlap`
  (params (OverlappedComponent :type "PrimitiveComponent Object Reference") (OtherActor :type "Actor Object Reference") (OtherComp :type "PrimitiveComponent Object Reference") (OtherBodyIndex :type Integer) (bFromSweep :type Boolean) (SweepResult :type "HitResult Structure (by ref)"))
  (`self.EnableInput` (`GameplayStatics.GetPlayerController` 0))
  (`KismetSystemLibrary.PrintString` "press e to place the fuse in this socket"))

(event `self.ReceiveBeginPlay`
  (`SceneComponent.K2_AddLocalRotation` (`self.fuseMesh`) (`self.TempRotator`) false false))

(event `self.Box.OnComponentEndOverlap`
  (params (OverlappedComponent :type "PrimitiveComponent Object Reference") (OtherActor :type "Actor Object Reference") (OtherComp :type "PrimitiveComponent Object Reference") (OtherBodyIndex :type Integer))
  (`self.DisableInput` (`GameplayStatics.GetPlayerController` 0))
  (`SceneComponent.SetVisibility` (`self.fuseMesh`) false false)
  (set `self.Rotations` 0)
  (`KismetSystemLibrary.PrintString` "player has exit socket"))

(event `self.ReceiveTick`
  (params (DeltaSeconds :type "Float (single-precision)"))
  (if (== (`self.Rotations`) 2)
    (bind _outactors (`GameplayStatics.GetAllActorsOfClass` null))
    (for _array_element _outactors
      (`self.Open Door` _array_element)
      (`PrimitiveComponent.SetMaterial` (`self.StaticMesh`) 0 null))))

(event `Key|E`
  (params (Key :type "Key Structure"))
  (:`Pressed`
    (bind _asfirst_person_character (cast `` (`Controller.K2_GetPawn` (`GameplayStatics.GetPlayerController` 0))))
    (if (== (`KismetArrayLibrary.Array_Length` (`/Game/MigratedA1/A1_Blueprints/Bp_FuseSocket.Fuses` _asfirst_person_character)) 1)
      (`SceneComponent.SetVisibility` (`self.fuseMesh`) true false)
      (set `self.fuseIsPlaced` true)
      (if (== (`self.fuseIsPlaced`) true)
        (`KismetSystemLibrary.PrintString` "press f to rotate the fuse"))
      (else
        (`KismetSystemLibrary.PrintString` "find the fuse first")))))

(event `Key|F`
  (params (Key :type "Key Structure"))
  (:`Pressed`
    (`self.rotateFuse90`)))

(fn `rotateFuse90`
  (if (== (`self.fuseIsPlaced`) true)
    (`SceneComponent.K2_AddLocalRotation` (`self.fuseMesh`) (struct :`Yaw` 90.0) false false)
    (`/Engine/EditorBlueprintResources/StandardMacros.IncrementInt` (`self.Rotations`))))

(fn `UserConstructionScript`)